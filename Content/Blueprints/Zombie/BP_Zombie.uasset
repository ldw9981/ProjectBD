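; BP_Zombie is a zombie Blueprint that displays its health on an attached widget.
; Every Tick it casts the widget's user object to UMG_ZombieHP and sets its Percent from CurrentHP divided by MaxHP.
; It then sets the widget's world pitch to the negated pitch of the first player controller's control rotation, with yaw and roll fixed at zero.
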(event EventBeginPlay)

(event Collision|EventActorBeginOverlap
  (params (OtherActor :type Actor%20Object%20Reference)))

(event EventTick
  (params (DeltaSeconds :type Float%20%28single-precision%29))
  (bind _asumg_zombie_hp (Utilities|Casting|CastToUMG_ZombieHP (UserInterface|GetUserWidgetObject (Variables|Default|GetWidget))))
  (Variables|/Game/Blueprints/Zombie/UI/UMG_ZombieHP.UMG_ZombieHP_C|SetPercent _asumg_zombie_hp (/ (Variables|Default|GetCurrentHP) (Variables|Default|GetMaxHP)))
  (Transformation|SetWorldRotation (Variables|Default|GetWidget) (Math|Rotator|MakeRotator 0.0 (* (.pitch (Pawn|GetControlRotation (Game|GetPlayerController 0) :!class /Script/Engine.Controller)) -1.0) 0.0) false false))

(fn ConstructionScript)